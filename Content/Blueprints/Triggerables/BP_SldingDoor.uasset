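; BP_SldingDoor is a triggerable double sliding door that opens on its Overlap event and closes on Unoverlapped.
; Overlap plays a timeline whose DoorOpenAmount lerps the relative locations of the left and right meshes from fixed closed offsets to per-door open-position variables.
; Unoverlapped reverses the same timeline.
; The actor does no overlap detection in its graph, as its own overlap event is disabled.
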(event `self.Overlap`
  (params (`Other Actor` :type "Actor Object Reference"))
  (bind (_direction _door_open_amount) (`Timeline|Timeline` :!label _label)
    (:`Update`
      (`SceneComponent.K2_SetRelativeLocation` (`self.SM_DoorLeft`) (`KismetMathLibrary.VLerp` (0.0 -180.0 0.0) (`self.L_DoorOpenPos`) _door_open_amount) false false)
      (`SceneComponent.K2_SetRelativeLocation` (`self.SM_DoorRight`) (`KismetMathLibrary.VLerp` (0.0 180.0 0.0) (`self.R_DoorOpenPos`) _door_open_amount) false false))))

(event `self.Unoverlapped`
  (params (`Other Actor` :type "Actor Object Reference"))
  (goto _label :!via `Reverse`))

(fn `UserConstructionScript`
  (`parent.UserConstructionScript`))